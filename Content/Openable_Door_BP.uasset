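; Openable door actor that swings open and closed when its OpenDoor component or interface raises open and close requests.
; It stores its initial rotation at BeginPlay, then a timeline's open angle adds a yaw offset to that rotation on each update.
; Close requests reverse the same timeline, and a sound timing event on the timeline plays a door lock sound at the actor's location.
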(event `self.ReceiveBeginPlay`
  ;[1 1 1] Set initial rotation
  (set `self.InitialRotation` (`self.K2_GetActorRotation`)))

(event `self.OpenDoor.OnOpenRequest`
  ;[1 1 1] Door Rotation
  (bind (_direction _openangle) (`Timeline|OpenTimeline` :!label _label)
    (:`Update`
      (`self.K2_SetActorRotation` (`KismetMathLibrary.ComposeRotators` (`self.InitialRotation`) (`KismetMathLibrary.MakeRotator` 0.0 0.0 _openangle))))
    (:`Sound Timing`
      (`GameplayStatics.PlaySoundAtLocation` "/Game/Audio/door-lock.door-lock" (`self.K2_GetActorLocation`) (struct) 1.0 1.0 0.0 null null null))))

(event `self.OpenDoor.OnCloseRequest`
  ;[1 1 1] Door Rotation
  (goto _label :!via `Reverse`))

(fn `UserConstructionScript`)